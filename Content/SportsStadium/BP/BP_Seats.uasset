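; Procedural stadium seating Blueprint that fills a stand with instances of a chosen mesh, built entirely in the construction script.
; It offsets SplineColumn1's two endpoints to shape SplineColumn2, then stretches up to 22 row splines between evenly spaced points on both.
; A Hierarchical Instanced Static Mesh places yaw-aligned seats along each row, using per-row counts and spacing offsets, with the last seat pinned to the spline's end.
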(event EventBeginPlay)

(event Collision|EventActorBeginOverlap
  (params (OtherActor :type Actor%20Object%20Reference)))

(event EventTick
  (params (DeltaSeconds :type Float%20%28single-precision%29)))

(fn ConstructionScript
  (bind _splinecolumn1 (Variables|Default|GetSplineColumn1))
  (bind _splinecolumn2 (Variables|Default|GetSplineColumn2))
  (bind _hierarchicalinstancedstaticmesh (Variables|Default|GetHierarchicalInstancedStaticMesh))
  (Components|StaticMesh|SetStaticMesh (Variables|Default|GetHierarchicalInstancedStaticMesh) (Variables|Default|GetMesh)) ; Set the static mesh for the base of the legs
  (Variables|Default|SetRawSplines (Utilities|Array|MakeArray (Variables|Default|GetSplineRaw_0) (Variables|Default|GetSplineRaw_1) (Variables|Default|GetSplineRaw_2) (Variables|Default|GetSplineRaw_3) (Variables|Default|GetSplineRaw_4) (Variables|Default|GetSplineRaw_5) (Variables|Default|GetSplineRaw_6) (Variables|Default|GetSplineRaw_7) (Variables|Default|GetSplineRaw_8) (Variables|Default|GetSplineRaw_9) (Variables|Default|GetSplineRaw_10) (Variables|Default|GetSplineRaw_11) (Variables|Default|GetSplineRaw_12) (Variables|Default|GetSplineRaw_13) (Variables|Default|GetSplineRaw_14) (Variables|Default|GetSplineRaw_15) (Variables|Default|GetSplineRaw_16) (Variables|Default|GetSplineRaw_17) (Variables|Default|GetSplineRaw_18) (Variables|Default|GetSplineRaw_19) (Variables|Default|GetSplineRaw_20) (Variables|Default|GetSplineRaw_21)))
  (Spline|SetLocationatSplinePoint (Variables|Default|GetSplineColumn2) 0 (+ (Spline|GetLocationatSplinePoint (Variables|Default|GetSplineColumn1) 0 "Local") (Variables|Default|GetOfssetColumnPoint0)) "Local" true)
  (Spline|SetLocationatSplinePoint (Variables|Default|GetSplineColumn2) 1 (+ (Spline|GetLocationatSplinePoint (Variables|Default|GetSplineColumn1) 1 "Local") (Variables|Default|GetOfssetColumnPoint1)) "Local" true)
  (for _index (range 0 (Variables|Default|GetColumn))
    (Variables|Default|SetColumnIndex _index)
    (Spline|SetLocationatSplinePoint (Utilities|Array|Get(acopy) (Variables|Default|GetRawSplines) (Variables|Default|GetColumnIndex)) 0 (Spline|GetLocationatDistanceAlongSpline _splinecolumn1 (* (/ (Math|Conversions|ToFloat(Integer) _index) (Math|Conversions|ToFloat(Integer) (Variables|Default|GetColumn))) (Spline|GetSplineLength _splinecolumn1)) "Local") "Local" true)
    (Spline|SetLocationatSplinePoint (Utilities|Array|Get(acopy) (Variables|Default|GetRawSplines) (Variables|Default|GetColumnIndex)) 1 (Spline|GetLocationatDistanceAlongSpline _splinecolumn2 (* (/ (Math|Conversions|ToFloat(Integer) _index) (Math|Conversions|ToFloat(Integer) (Variables|Default|GetColumn))) (Spline|GetSplineLength _splinecolumn2)) "Local") "Local" true)
    (for _index_2 (range 0 (Utilities|Array|Get(acopy) (Variables|Default|GetRaws) (Variables|Default|GetColumnIndex))) ; Loop through each road section, offset by Leg Start and Leg End amounts set by the user
      (bind _output_get (Variables|Default|SetLocal_CurrentIndex _index_2))
      (if (!= _output_get (Utilities|Array|Get(acopy) (Variables|Default|GetRaws) (Variables|Default|GetColumnIndex)))
        (Components|InstancedStaticMesh|AddInstance _hierarchicalinstancedstaticmesh (Math|Transform|MakeTransform (Spline|GetLocationatDistanceAlongSpline (Utilities|Array|Get(acopy) (Variables|Default|GetRawSplines) (Variables|Default|GetColumnIndex)) (* (Variables|Default|GetLocal_CurrentIndex) (+ (Variables|Default|GetSpacing) (Utilities|Array|Get(acopy) (Variables|Default|GetSpacing_Offset) (Variables|Default|GetColumnIndex)))) "Local") (Math|Rotator|MakeRotator 0.0 0.0 (.yaw (Spline|GetRotationatDistanceAlongSpline (Utilities|Array|Get(acopy) (Variables|Default|GetRawSplines) (Variables|Default|GetColumnIndex)) (* (Variables|Default|GetLocal_CurrentIndex) (+ (Variables|Default|GetSpacing) (Utilities|Array|Get(acopy) (Variables|Default|GetSpacing_Offset) (Variables|Default|GetColumnIndex)))) "Local")))))
        (else
          (Components|InstancedStaticMesh|AddInstance _hierarchicalinstancedstaticmesh (Math|Transform|MakeTransform (Spline|GetLocationatDistanceAlongSpline (Utilities|Array|Get(acopy) (Variables|Default|GetRawSplines) (Variables|Default|GetColumnIndex)) (Spline|GetSplineLength (Utilities|Array|Get(acopy) (Variables|Default|GetRawSplines) (Variables|Default|GetColumnIndex))) "Local") (Math|Rotator|MakeRotator 0.0 0.0 (.yaw (Spline|GetRotationatDistanceAlongSpline (Utilities|Array|Get(acopy) (Variables|Default|GetRawSplines) (Variables|Default|GetColumnIndex)) (Spline|GetSplineLength (Utilities|Array|Get(acopy) (Variables|Default|GetRawSplines) (Variables|Default|GetColumnIndex))) "Local"))))))))))